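; BP_Tunnel is a tunnel segment with a rotating holed wall, an offset enemy and a pickup that spawns half the time.
; RandomizeWall picks one of four hole meshes, a random roll and a random-colored dynamic material, while BreakWall removes the wall.
; Wall hits call TakeHitWall on the player and set WasHit.
; The trigger awards score if the wall was not hit, asks TunnelSpawner for the next tunnel, then destroys this one.
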(event `self.ReceiveBeginPlay`
  (bind _pickup (`self.Pickup`))
  (bind _enemy (`self.Enemy`))
  (`|ExecutionSequence`
    (:`then_0`
      (if (`KismetMathLibrary.RandomBoolWithWeight` 0.0)
        (`ActorComponent.K2_DestroyComponent` _enemy)
        (else
          (`SceneComponent.K2_AddLocalOffset` _enemy (* (`KismetMathLibrary.RandomUnitVector`) (400.0 400.0 0.0)) false true))))
    (:`then_1`
      (if (`KismetMathLibrary.RandomBoolWithWeight` 0.5)
        (`ActorComponent.K2_DestroyComponent` _pickup)
        (else
          (`SceneComponent.K2_AddLocalOffset` _pickup (* (`KismetMathLibrary.RandomUnitVector`) (400.0 400.0 0.0)) false true))))))

(event `self.ReceiveTick`
  (params (DeltaSeconds :type "Float (single-precision)"))
  (bind _wall_mesh (`self.Wall Mesh`))
  (`/Engine/EditorBlueprintResources/StandardMacros.IsValid` _wall_mesh
    (:`Is Valid`
      (`SceneComponent.K2_AddLocalRotation` _wall_mesh (`KismetMathLibrary.MakeRotator` (* DeltaSeconds (`self.RotateSpeed`))) false false))))

(event `self.TriggerZone.OnComponentBeginOverlap`
  (params (OverlappedComponent :type "PrimitiveComponent Object Reference") (OtherActor :type "Actor Object Reference") (OtherComp :type "PrimitiveComponent Object Reference") (OtherBodyIndex :type Integer) (bFromSweep :type Boolean) (SweepResult :type "HitResult Structure (by ref)"))
  (bind _asbp_player (cast `/Game/InfiniteMatrix/Blueprints/BP_Player` OtherActor))
  (if (not (`self.WasHit`))
    (`/Game/InfiniteMatrix/Blueprints/BP_Player.inc score` _asbp_player))
  (`/Game/InfiniteMatrix/Blueprints/BP_TunnelSpawner.SpawnTunnelAtSpawnPoint` (`self.TunnelSpawner`))
  (`self.K2_DestroyActor`))

(event `self.Wall Mesh.OnComponentHit`
  (params (HitComponent :type "PrimitiveComponent Object Reference") (OtherActor :type "Actor Object Reference") (OtherComp :type "PrimitiveComponent Object Reference") (NormalImpulse :type "Vector Structure") (Hit :type "HitResult Structure (by ref)"))
  (bind _asbp_player (cast `/Game/InfiniteMatrix/Blueprints/BP_Player` OtherActor))
  (`/Game/InfiniteMatrix/Blueprints/BP_Player.take hit wall` _asbp_player self)
  (set `self.WasHit` true))

(fn `break wall`
  (`ActorComponent.K2_DestroyComponent` (`self.Wall Mesh`)))

(fn `Randomize Wall`
  (`StaticMeshComponent.SetStaticMesh` (`self.Wall Mesh`) (select `int` (`KismetMathLibrary.RandomIntegerInRange` 0 3) :`0` "/Game/InfiniteMatrix/Meshes/SM_Hole_01.SM_Hole_01" :`1` "/Game/InfiniteMatrix/Meshes/SM_Hole_02.SM_Hole_02" :`2` "/Game/InfiniteMatrix/Meshes/SM_Hole_03.SM_Hole_03" :`3` "/Game/InfiniteMatrix/Meshes/SM_Hole_04.SM_Hole_04" :!type "StaticMesh Object Reference"))
  (`SceneComponent.K2_AddLocalRotation` (`self.Wall Mesh`) (`KismetMathLibrary.MakeRotator` (`KismetMathLibrary.RandomFloatInRange` 0.0 360.0)) false false)
  (bind _returnvalue (`KismetMaterialLibrary.CreateDynamicMaterialInstance` "/Game/InfiniteMatrix/Materials/MI_Hole.MI_Hole"))
  (`MaterialInstanceDynamic.SetVectorParameterValue` _returnvalue "Color" (`KismetMathLibrary.Conv_VectorToLinearColor` (+ (* (`KismetMathLibrary.RandomUnitVector`) (0.5 0.5 0.5)) (0.5 0.5 0.5))))
  (`PrimitiveComponent.SetMaterial` (`self.Wall Mesh`) 0 _returnvalue))

(fn `UserConstructionScript`)
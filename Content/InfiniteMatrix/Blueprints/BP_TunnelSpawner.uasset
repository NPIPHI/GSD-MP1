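; BP_TunnelSpawner builds a chain of randomized BP_Tunnel segments for the Infinite Matrix level.
; On BeginPlay it destroys existing tunnels, then spawns a short initial run starting at the player pawn's location.
; Each new segment attaches at the newest tunnel's SpawnPoint, randomizes its walls and becomes NewestTunnel.
; Tunnels receive a reference back to the spawner, and SpawnTunnelAtSpawnPoint extends the chain by one segment.
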(event `self.ReceiveBeginPlay`
  (`self.SpawnInitalTunnels`))

(fn `SpawnInitalTunnels`
  (`|ExecutionSequence`
    (:`then_0`
      (bind _outactors (`GameplayStatics.GetAllActorsOfClass` "/Game/InfiniteMatrix/Blueprints/BP_Tunnel.BP_Tunnel_C"))
      (for _array_element _outactors
        (`self.K2_DestroyActor` _array_element)))
    (:`then_1`
      (for _ (range 3)
        (`/Engine/EditorBlueprintResources/StandardMacros.IsValid` (`self.Newest Tunnel`)
          (:`Is Valid`
            (`self.SpawnTunnelAtSpawnPoint`))
          (:`Is Not Valid`
            (bind _tunnel (`self.SpawnTunnel` (`self.K2_GetActorLocation` (`GameplayStatics.GetPlayerPawn` 0))))
            (bind _output_get (set `self.Newest Tunnel` _tunnel))
            (set `/Game/InfiniteMatrix/Blueprints/BP_Tunnel.TunnelSpawner` self _output_get)))))))

(fn `SpawnTunnel`
  (params (SpawnLoacation :type "Vector Structure"))
  (returns (Tunnel :type "/Game/InfiniteMatrix/Blueprints/BP_Tunnel Object Reference"))
  (bind _returnvalue (`|SpawnActorFromClass` "/Game/InfiniteMatrix/Blueprints/BP_Tunnel.BP_Tunnel_C" (`KismetMathLibrary.MakeTransform` SpawnLoacation) "Undefined" "MultiplyWithRoot" null null))
  (`/Game/InfiniteMatrix/Blueprints/BP_Tunnel.Randomize Wall` _returnvalue)
  (return _returnvalue))

(fn `SpawnTunnelAtSpawnPoint`
  (bind _tunnel (`self.SpawnTunnel` (`SceneComponent.K2_GetComponentLocation` (`/Game/InfiniteMatrix/Blueprints/BP_Tunnel.SpawnPoint` (`self.Newest Tunnel`)))))
  (bind _output_get (set `self.Newest Tunnel` _tunnel))
  (set `/Game/InfiniteMatrix/Blueprints/BP_Tunnel.TunnelSpawner` self _output_get))

(fn `UserConstructionScript`)
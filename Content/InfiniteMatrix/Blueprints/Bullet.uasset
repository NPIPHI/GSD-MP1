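; Bullet is a projectile actor that spins around its roll axis as it flies at a velocity assigned through SetVel.
; Each tick it moves with a swept world offset and counts down Lifetime, destroying itself once that drops below zero.
; Overlapping anything other than BP_Player zeroes Lifetime, so removal happens through the same Tick check, while player overlaps are ignored.
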(event `self.ReceiveTick`
  (params (DeltaSeconds :type "Float (single-precision)"))
  (`|ExecutionSequence`
    (:`then_0`
      (`self.K2_AddActorLocalRotation` (`KismetMathLibrary.MakeRotator` (* DeltaSeconds 360.0))))
    (:`then_1`
      (`self.K2_AddActorWorldOffset` (* DeltaSeconds (`self.Vel`)) true)
      (bind _output_get (set `self.Lifetime` (- (`self.Lifetime`) DeltaSeconds)))
      (`/Engine/EditorBlueprintResources/StandardMacros.CompareFloat` _output_get
        (:`<`
          (`self.K2_DestroyActor`))))))

(event `self.Bullet.OnComponentBeginOverlap`
  (params (OverlappedComponent :type "PrimitiveComponent Object Reference") (OtherActor :type "Actor Object Reference") (OtherComp :type "PrimitiveComponent Object Reference") (OtherBodyIndex :type Integer) (bFromSweep :type Boolean) (SweepResult :type "HitResult Structure (by ref)"))
  (cast `/Game/InfiniteMatrix/Blueprints/BP_Player` OtherActor
    (:`CastFailed`
      (set `self.Lifetime` 0.0))))

(fn `Set Vel`
  (params (Vel :type "Vector Structure"))
  (set `self.Vel` Vel))

(fn `UserConstructionScript`)